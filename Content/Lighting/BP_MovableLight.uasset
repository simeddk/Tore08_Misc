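; BP_MovableLight is an actor that moves continuously in a horizontal circle around its spawn point, likely carrying a light.
; BeginPlay stores the start location.
; Each Tick offsets it by sine and cosine of game time with a fixed radius, setting the location without sweep, so height stays constant.
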(event `self.ReceiveBeginPlay`
  (set `self.Start` (`self.K2_GetActorLocation`)))

(event `self.ReceiveTick`
  (params (DeltaSeconds :type "Float (single-precision)"))
  (bind _returnvalue (`GameplayStatics.GetTimeSeconds`))
  (`self.K2_SetActorLocation` (+ (`self.Start`) (`KismetMathLibrary.MakeVector` (* 150 (`KismetMathLibrary.Sin` _returnvalue)) (* 150 (`KismetMathLibrary.Cos` _returnvalue))))))

(fn `UserConstructionScript`)